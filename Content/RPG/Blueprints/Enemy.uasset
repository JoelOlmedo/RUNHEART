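; Enemy Blueprint in an RPG that lets the player interact with it by pressing E inside an overlap zone.
; Entering the Interact component's overlap shows a prompt widget and sets CanInteract; leaving removes all widgets and clears the flag.
; Pressing E while the flag is set swaps all widgets for a Text widget.
; A fade and level-load sequence to FirstPersonMap is unconnected, and the Box overlap event is empty.
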(event `Key|E`
  (params (Key :type "Key Structure"))
  (:`Pressed`
    (if (`self.CanInteract`)
      (`KismetSystemLibrary.PrintText` "E")
      (`WidgetLayoutLibrary.RemoveAllWidgets`)
      (bind _returnvalue (`|CreateWidget` "/Game/RPG/Widget/Text.Text_C"))
      (`UserWidget.AddToViewport` _returnvalue 0))))

(event `self.Box.OnComponentBeginOverlap`
  (params (OverlappedComponent :type "PrimitiveComponent Object Reference") (OtherActor :type "Actor Object Reference") (OtherComp :type "PrimitiveComponent Object Reference") (OtherBodyIndex :type Integer) (bFromSweep :type Boolean) (SweepResult :type "HitResult Structure (by ref)")))

(event `self.Interact.OnComponentBeginOverlap`
  (params (OverlappedComponent :type "PrimitiveComponent Object Reference") (OtherActor :type "Actor Object Reference") (OtherComp :type "PrimitiveComponent Object Reference") (OtherBodyIndex :type Integer) (bFromSweep :type Boolean) (SweepResult :type "HitResult Structure (by ref)"))
  (bind _returnvalue (`|CreateWidget` "/Game/RPG/Widget/Interact.Interact_C"))
  (`UserWidget.AddToViewport` _returnvalue 0)
  (set `self.CanInteract` true))

(event `self.Interact.OnComponentEndOverlap`
  (params (OverlappedComponent :type "PrimitiveComponent Object Reference") (OtherActor :type "Actor Object Reference") (OtherComp :type "PrimitiveComponent Object Reference") (OtherBodyIndex :type Integer))
  (`WidgetLayoutLibrary.RemoveAllWidgets`)
  (set `self.CanInteract` false))

(fn `UserConstructionScript`)