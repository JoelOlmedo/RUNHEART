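; An overworld trigger that shows a level's saved time and earned medals while the player stands inside its box.
; On BeginPlay it creates a hidden results widget, loads the time and medal thresholds from a data file named after its Level number, and awards medals cumulatively.
; The widget only gets its level name, time and refresh when a saved time exists.
; Overlap toggles visibility, with a timeline scaling the widget in on entry.
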(event `self.ReceiveBeginPlay`
  (bind _timeloader (`self.TimeLoader`))
  (bind _widget (`self.Widget`))
  (bind _widget_2 (`self.Widget`))
  (bind _widget_3 (`self.Widget`))
  (bind _returnvalue (`|CreateWidget` "/Game/UI/Widgets/Overworld_Results.Overworld_Results_C"))
  (bind _output_get (set `self.Widget` _returnvalue))
  (`UserWidget.AddToViewport` _output_get 0)
  (`Widget.SetVisibility` (`self.Widget`) "Hidden")
  (set `/Game/FirstPerson/Blueprints/TimeLoad/TimeLoader.Data File` (`KismetStringLibrary.BuildString_Int` "" "Level_" (`self.Level`) "_Times") (`self.TimeLoader`))
  (bind _time (`/Game/FirstPerson/Blueprints/TimeLoad/TimeLoader.LoadTime` _timeloader))
  (bind (_bronzetime _silvertime _goldtime) (`/Game/FirstPerson/Blueprints/TimeLoad/TimeLoader.LoadMedals` _timeloader))
  (bind _output_get_2 (set `/Game/UI/Widgets/Overworld_Results.BronzeTime` _bronzetime _widget_2))
  (bind _output_get_3 (set `/Game/UI/Widgets/Overworld_Results.SilverTime` _silvertime _widget_2))
  (bind _output_get_4 (set `/Game/UI/Widgets/Overworld_Results.GoldTime` _goldtime _widget_2))
  (if (not (== _time 0.0))
    (if (> _output_get_4 _time)
      (set `/Game/UI/Widgets/Overworld_Results.GoldMedal` true _widget)
      (set `/Game/UI/Widgets/Overworld_Results.SilverMedal` true _widget :!label _label)
      (set `/Game/UI/Widgets/Overworld_Results.BronzeMedal` true _widget :!label _label_2)
      (elif (> _output_get_3 _time)
        (goto _label)
        (elif (> _output_get_2 _time)
          (goto _label_2)
          (else
            _))))
    (bind _output_get_5 (set `/Game/UI/Widgets/Overworld_Results.LevelName` (`KismetStringLibrary.Concat_StrStr` "Level " (`KismetStringLibrary.Conv_IntToString` (`self.Level`))) _widget_3))
    (`KismetSystemLibrary.PrintString` _output_get_5)
    (set `/Game/UI/Widgets/Overworld_Results.MaxTime` _time _widget_3)
    (`/Game/UI/Widgets/Overworld_Results.Update` _widget_3)))

(event `self.Box.OnComponentBeginOverlap`
  (params (OverlappedComponent :type "PrimitiveComponent Object Reference") (OtherActor :type "Actor Object Reference") (OtherComp :type "PrimitiveComponent Object Reference") (OtherBodyIndex :type Integer) (bFromSweep :type Boolean) (SweepResult :type "HitResult Structure (by ref)"))
  (bind _widget (`self.Widget`))
  (cast `/Game/RPG/Personaje/Player` OtherActor)
  (`Widget.SetVisibility` _widget "Visible")
  (bind (_direction _scale) (`Timeline|Timeline` :!via `PlayFromStart`)
    (:`Update`
      (set `Widget.RenderTransform` (make `WidgetTransform` (0.0 0.0) (`KismetMathLibrary.MakeVector2D` _scale _scale)) _widget))))

(event `self.Box.OnComponentEndOverlap`
  (params (OverlappedComponent :type "PrimitiveComponent Object Reference") (OtherActor :type "Actor Object Reference") (OtherComp :type "PrimitiveComponent Object Reference") (OtherBodyIndex :type Integer))
  (cast `/Game/RPG/Personaje/Player` OtherActor)
  (`Widget.SetVisibility` (`self.Widget`) "Hidden"))

(fn `UserConstructionScript`)