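; Town manager that tracks the game phase and opens the town level matching it.
; On BeginPlay it has its Loader load the phase and copies it into GamePhase.
; Loading the town appends GamePhase to a base level name and opens that level by name.
; ResetGame calls the Loader's SavePhase, then zeroes the local GamePhase.
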(event `self.ReceiveBeginPlay`
  (`/Game/RPG/Blueprints/Saver/TownLoader.LoadPhase` (`self.Loader`))
  (set `self.GamePhase` (`/Game/RPG/Blueprints/Saver/TownLoader.Phase` (`self.Loader`))))

(event `ResetGame`
  (`/Game/RPG/Blueprints/Saver/TownLoader.SavePhase` (`self.Loader`))
  (set `self.GamePhase` 0))

(event `LoadTownLevel`
  (`GameplayStatics.OpenLevel` (`KismetStringLibrary.Conv_StringToName` (`KismetStringLibrary.BuildString_Int` (`KismetStringLibrary.Conv_NameToString` (`self.levelName`)) "" (`self.GamePhase`)))))

(fn `UserConstructionScript`)