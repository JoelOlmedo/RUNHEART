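; TownLoader saves and loads the RPG's game Phase value through a GamePhaseDataSave object in the DataFile save slot.
; SaveOnce writes the current Phase only when no save exists yet, while SavePhase loads or creates the save object and overwrites its Phase.
; LoadPhase copies the stored Phase back into the Blueprint's variable, leaving it unchanged if no save exists.
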(event `SaveOnce`
  (bind _data_file (`self.Data File`))
  (bind _returnvalue (`GameplayStatics.DoesSaveGameExist` _data_file))
  (if (not _returnvalue)
    (bind _returnvalue_2 (`GameplayStatics.CreateSaveGameObject` "/Game/RPG/Blueprints/Saver/GamePhaseDataSave.GamePhaseDataSave_C"))
    (bind _output_get (set `self.SaveREF` _returnvalue_2))
    (bind _asgame_phase_data_save (cast `/Game/RPG/Blueprints/Saver/GamePhaseDataSave` _output_get))
    (set `/Game/RPG/Blueprints/Saver/GamePhaseDataSave.Phase` (`self.Phase`) _asgame_phase_data_save)
    (`GameplayStatics.SaveGameToSlot` (`self.SaveREF`) _data_file)))

(event `SavePhase`
  (bind _data_file (`self.Data File`))
  (bind _returnvalue (`GameplayStatics.DoesSaveGameExist` _data_file))
  (if _returnvalue
    (bind _returnvalue_2 (`GameplayStatics.LoadGameFromSlot` _data_file))
    (set `self.SaveREF` _returnvalue_2)
    (else
      (bind _returnvalue_3 (`GameplayStatics.CreateSaveGameObject` "/Game/RPG/Blueprints/Saver/GamePhaseDataSave.GamePhaseDataSave_C"))
      (bind _output_get (set `self.SaveREF` _returnvalue_3))))
  (bind _asgame_phase_data_save (cast `/Game/RPG/Blueprints/Saver/GamePhaseDataSave` _output_get))
  (set `/Game/RPG/Blueprints/Saver/GamePhaseDataSave.Phase` (`self.Phase`) _asgame_phase_data_save)
  (`GameplayStatics.SaveGameToSlot` (`self.SaveREF`) _data_file))

(event `LoadPhase`
  (bind _data_file (`self.Data File`))
  (bind _returnvalue (`GameplayStatics.DoesSaveGameExist` _data_file))
  (if _returnvalue
    (bind _returnvalue_2 (`GameplayStatics.LoadGameFromSlot` _data_file))
    (bind _asgame_phase_data_save (cast `/Game/RPG/Blueprints/Saver/GamePhaseDataSave` _returnvalue_2))
    (set `self.Phase` (`/Game/RPG/Blueprints/Saver/GamePhaseDataSave.Phase` _asgame_phase_data_save))))