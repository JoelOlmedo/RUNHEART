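; TrainingTransition sets which level the game moves to next, based on the saved game phase.
; On BeginPlay it has its Loader load the phase and stores the result in GamePhase.
; It appends that number to the LevelName base and writes the resulting name into LevelToGo on the NextLevel actor found in the world.
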(event `self.ReceiveBeginPlay`
  (`/Game/RPG/Blueprints/Saver/TownLoader.LoadPhase` (`self.Loader`))
  (set `self.GamePhase` (`/Game/RPG/Blueprints/Saver/TownLoader.Phase` (`self.Loader`)))
  (bind _returnvalue (`GameplayStatics.GetActorOfClass` "/Game/RPG/Blueprints/NextLevel.NextLevel_C"))
  (set `/Game/RPG/Blueprints/NextLevel.LevelToGo` (`KismetStringLibrary.Conv_StringToName` (`KismetStringLibrary.BuildString_Int` (`KismetStringLibrary.Conv_NameToString` (`self.levelName`)) "" (`self.GamePhase`))) _returnvalue))

(fn `UserConstructionScript`)