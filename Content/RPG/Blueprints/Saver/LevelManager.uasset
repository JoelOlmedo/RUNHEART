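; Level manager actor that applies saved town progress and player spawn position when play begins.
; It reads the saved phase from TownLoader and destroys every actor tagged "Level" plus a number, for each number from 1 up to that phase.
; It then asks SpawnRPGLoader for a saved location and moves the Player there without sweeping, only if that location is valid.
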(event `self.ReceiveBeginPlay`
  (`|ExecutionSequence`
    (:`then_0`
      (bind _phase (`/Game/RPG/Blueprints/Saver/TownLoader.LoadPhase` (`self.TownLoader`)))
      (for _index (range 1 (+ _phase 1))
        (bind _outactors (`GameplayStatics.GetAllActorsWithTag` (`KismetStringLibrary.Conv_StringToName` (`KismetStringLibrary.Concat_StrStr` "Level" (`KismetStringLibrary.Conv_IntToString` _index)))))
        (for _array_element _outactors
          (`self.K2_DestroyActor` _array_element))))
    (:`then_1`
      (bind _returnvalue (`GameplayStatics.GetActorOfClass` "/Game/RPG/Personaje/Player.Player_C"))
      (bind (_location _valid) (`/Game/RPG/Blueprints/Saver/Respawn/SpawnRPGLoader.LoadLocation` (`self.SpawnRPGLoader`)))
      (if _valid
        (`self.K2_SetActorLocation` _returnvalue _location false false)))))

(fn `UserConstructionScript`)