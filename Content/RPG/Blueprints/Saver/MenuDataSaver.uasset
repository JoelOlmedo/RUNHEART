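; Menu data saver Blueprint that seeds and resets persistent game data through town, time and spawn loader members.
; BeginPlay calls the town SaveOnce and writes bronze, silver and gold medal thresholds for ten levels via SetLevelMedals.
; ResetGame saves a town phase, zeroes each level's time and saves a zero spawn location.
; TimeLoader is retargeted per level by building its data file name from the index.
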(event `self.ReceiveBeginPlay`
  (`/Game/RPG/Blueprints/Saver/TownLoader.SaveOnce` (`self.TownLoader`) 0)
  (`self.SetLevelMedals` 1 95.0 75.0 60.0)
  (`self.SetLevelMedals` 2 90.0 70.0 55.0)
  (`self.SetLevelMedals` 3 90.0 70.0 55.0)
  (`self.SetLevelMedals` 4 90.0 70.0 55.0)
  (`self.SetLevelMedals` 5 105.0 85.0 70.0)
  (`self.SetLevelMedals` 6 100.0 80.0 65.0)
  (`self.SetLevelMedals` 7 115.0 95.0 80.0)
  (`self.SetLevelMedals` 8 100.0 80.0 65.0)
  (`self.SetLevelMedals` 9 100.0 80.0 65.0)
  (`self.SetLevelMedals` 10 110.0 90.0 75.0))

(event `Reset Game`
  (bind _timeloader (`self.TimeLoader`))
  (`/Game/RPG/Blueprints/Saver/TownLoader.SavePhase` (`self.TownLoader`) 2)
  (for _index (range 1 11)
    (set `/Game/FirstPerson/Blueprints/TimeLoad/TimeLoader.Data File` (`KismetStringLibrary.BuildString_Int` "" "Level_" _index "_Times") _timeloader)
    (`/Game/FirstPerson/Blueprints/TimeLoad/TimeLoader.SaveTime` _timeloader 0.0)
    (`/Game/RPG/Blueprints/Saver/Respawn/SpawnRPGLoader.SaveLocation` (`self.SpawnRPGLoader`) (0.0 0.0 0.0))))

(fn `SetLevelMedals`
  (params (Lvl :type Integer) (Bronze :type "Float (double-precision)") (Silver :type "Float (double-precision)") (Gold :type "Float (double-precision)"))
  (bind _timeloader (`self.TimeLoader`))
  (set `/Game/FirstPerson/Blueprints/TimeLoad/TimeLoader.Data File` (`KismetStringLibrary.BuildString_Int` "" "Level_" Lvl "_Times") _timeloader)
  (`/Game/FirstPerson/Blueprints/TimeLoad/TimeLoader.SaveMedals` _timeloader Bronze Silver Gold))

(fn `UserConstructionScript`)