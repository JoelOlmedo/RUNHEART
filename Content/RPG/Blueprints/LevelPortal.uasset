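; A level portal that sends the player to a numbered level when they overlap its collision.
; On BeginPlay it loads a phase number through a PhaseLoader and stores it as the next level index.
; On overlap by a Player, it appends that number to a base level name and opens the level by that name.
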(event `self.ReceiveBeginPlay`
  (bind _phaseloader (`self.PhaseLoader`))
  (`/Game/RPG/Blueprints/Saver/TownLoader.LoadPhase` _phaseloader)
  (set `self.NextLevel` (`/Game/RPG/Blueprints/Saver/TownLoader.Phase` _phaseloader)))

(event `self.Col.OnComponentBeginOverlap`
  (params (OverlappedComponent :type "PrimitiveComponent Object Reference") (OtherActor :type "Actor Object Reference") (OtherComp :type "PrimitiveComponent Object Reference") (OtherBodyIndex :type Integer) (bFromSweep :type Boolean) (SweepResult :type "HitResult Structure (by ref)"))
  (cast `/Game/RPG/Personaje/Player` OtherActor)
  (`GameplayStatics.OpenLevel` (`KismetStringLibrary.Conv_StringToName` (`KismetStringLibrary.BuildString_Int` (`KismetStringLibrary.Conv_NameToString` (`self.Level Name`)) "" (`self.NextLevel`)))))

(fn `UserConstructionScript`)